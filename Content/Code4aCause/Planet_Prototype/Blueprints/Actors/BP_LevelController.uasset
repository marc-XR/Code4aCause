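; BP_LevelController is a hidden launch pad that unlocks once the player has gathered every collectable in the level.
; It counts the assigned collectables at start and, when the collected count matches, reveals itself and plays an armed sound.
; Once armed, overlapping planet characters are launched upward and along the box's forward vector, and the MetaCharacter sound is triggered.
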(event `self.ReceiveBeginPlay`
  (set `self.CollectableCount` (`KismetArrayLibrary.Array_Length` (`self.Collectables`))))

(event `IncreaseCollectedCount`
  (bind _result (`/Engine/EditorBlueprintResources/StandardMacros.IncrementInt` (`self.CollectedCount`))
    (:`  `
      (if (== _result (`self.CollectableCount`))
        (`self.SetActorHiddenInGame` false)
        (set `self.Collected The Stuff_0` true)
        (`GameplayStatics.PlaySoundAtLocation` "/Game/Code4aCause/Audio/LaunchPad_armed_Draft__2wav.LaunchPad_armed_Draft__2wav" (0.0 0.0 0.0) (struct) 1.0 1.0 0.0 null null null null)))))

(event `self.ReceiveActorBeginOverlap`
  (params (OtherActor :type "Actor Object Reference"))
  (bind _meta_character (`self.Meta_Character`))
  (bind (_returnvalue_x _returnvalue_y) (`KismetMathLibrary.BreakVector` (* (`SceneComponent.GetForwardVector` (`self.Box`)) 1500.0)))
  (bind _asbp_planet_third_person_character_1 (cast `/Game/Code4aCause/Planet_Prototype/Blueprints/Characters/BP_Planet_ThirdPersonCharacter1` OtherActor))
  (if (`self.Collected The Stuff_0`)
    (`Character.LaunchCharacter` _asbp_planet_third_person_character_1 (`KismetMathLibrary.MakeVector` _returnvalue_x _returnvalue_y 3000.0) true false)
    (`AudioComponent.Play` _meta_character 0.0)
    (`AudioParameterControllerInterface.SetTriggerParameter` _meta_character "PlatformSound")))

(event `Collected the stuff`
  (params (`Collected the stuff` :type Boolean))
  (set `self.Collected The Stuff_0` `Collected the stuff`))

(fn `UserConstructionScript`)