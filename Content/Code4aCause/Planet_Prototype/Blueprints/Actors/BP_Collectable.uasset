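; BP_Collectable is a pickup actor that the planet third-person character collects by overlapping its collision component.
; The overlap plays a timeline that drives the world scale of separate uncollected and collected meshes to animate the change of state.
; When the timeline finishes, it sets Collected, then finds every BP_LevelController and increments the collected count on those whose Collectables list contains this actor.
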(event `self.CollectableCollision.OnComponentBeginOverlap`
  (params (OverlappedComponent :type "PrimitiveComponent Object Reference") (OtherActor :type "Actor Object Reference") (OtherComp :type "PrimitiveComponent Object Reference") (OtherBodyIndex :type Integer) (bFromSweep :type Boolean) (SweepResult :type "HitResult Structure (by ref)"))
  (bind _asbp_planet_third_person_character_1 (cast `/Game/Code4aCause/Planet_Prototype/Blueprints/Characters/BP_Planet_ThirdPersonCharacter1` OtherActor))
  (bind (_direction _scalevalue _collectedscale) (`Timeline|ScaleTimeline`)
    (:`Update`
      (`SceneComponent.SetWorldScale3D` (`self.UncollectedMesh`) (`KismetMathLibrary.Conv_DoubleToVector` _scalevalue))
      (`SceneComponent.SetWorldScale3D` (`self.CollectedMesh`) (`KismetMathLibrary.Conv_DoubleToVector` _collectedscale)))
    (:`Finished`
      (set `self.bCollected` true)
      (bind _outactors (`GameplayStatics.GetAllActorsOfClass` "/Game/Code4aCause/Planet_Prototype/Blueprints/Actors/BP_LevelController.BP_LevelController_C"))
      (for _array_element _outactors
        (if (`KismetArrayLibrary.Array_Contains` (`/Game/Code4aCause/Planet_Prototype/Blueprints/Actors/BP_LevelController.Collectables` _array_element) self)
          (`/Game/Code4aCause/Planet_Prototype/Blueprints/Actors/BP_LevelController.IncreaseCollectedCount` _array_element))))))

(fn `UserConstructionScript`)