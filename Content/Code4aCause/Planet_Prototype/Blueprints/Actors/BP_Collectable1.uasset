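; BP_Collectable1 is a two-stage planet collectable that is first found, then collected.
; CollectableCollision reacts to the player character, playing a sound and timeline that scales the uncollected and collected meshes, starts rotation and removes the uncollected mesh.
; CollectableCollision1 accepts any overlap without checking Found, playing a coin sound and marking Collected.
; It then increments the count on any BP_LevelController whose Collectables list matches and destroys the actor.
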(event `self.ReceiveBeginPlay`
  (`ActorComponent.Deactivate` (`self.RotatingMovement`)))

(event `self.CollectableCollision.OnComponentBeginOverlap`
  (params (OverlappedComponent :type "PrimitiveComponent Object Reference") (OtherActor :type "Actor Object Reference") (OtherComp :type "PrimitiveComponent Object Reference") (OtherBodyIndex :type Integer) (bFromSweep :type Boolean) (SweepResult :type "HitResult Structure (by ref)"))
  (if (not (`self.Found`))
    (bind _asbp_planet_third_person_character_1 (cast `/Game/Code4aCause/Planet_Prototype/Blueprints/Characters/BP_Planet_ThirdPersonCharacter1` OtherActor))
    (`GameplayStatics.PlaySoundAtLocation` "/Game/Code4aCause/Audio/Metasounds/Meta_Scale.Meta_Scale" (0.0 0.0 0.0) (struct) 1.0 1.0 0.0 null null null null)
    (bind (_direction _scalevalue _collectedscale) (`Timeline|ScaleTimeline`)
      (:`Update`
        (`SceneComponent.SetWorldScale3D` (`self.UncollectedMesh`) (`KismetMathLibrary.Conv_DoubleToVector` _scalevalue))
        (`SceneComponent.SetWorldScale3D` (`self.CollectedMesh`) (`KismetMathLibrary.Conv_DoubleToVector` _collectedscale))
        (set `self.Found` true)
        (`ActorComponent.Activate` (`self.RotatingMovement`) true))
      (:`Finished`
        (`ActorComponent.K2_DestroyComponent` (`self.UncollectedMesh`))))))

(event `self.CollectableCollision1.OnComponentBeginOverlap`
  (params (OverlappedComponent :type "PrimitiveComponent Object Reference") (OtherActor :type "Actor Object Reference") (OtherComp :type "PrimitiveComponent Object Reference") (OtherBodyIndex :type Integer) (bFromSweep :type Boolean) (SweepResult :type "HitResult Structure (by ref)"))
  (`GameplayStatics.PlaySoundAtLocation` "/Game/Code4aCause/Audio/Metasounds/Meta_Coin.Meta_Coin" (0.0 0.0 0.0) (struct) 1.0 1.0 0.0 null null null null)
  (set `self.bCollected` true)
  (bind _outactors (`GameplayStatics.GetAllActorsOfClass` "/Game/Code4aCause/Planet_Prototype/Blueprints/Actors/BP_LevelController.BP_LevelController_C"))
  (for _array_element _outactors
    (if (`KismetArrayLibrary.Array_Contains` (`/Game/Code4aCause/Planet_Prototype/Blueprints/Actors/BP_LevelController.Collectables` _array_element))
      (`/Game/Code4aCause/Planet_Prototype/Blueprints/Actors/BP_LevelController.IncreaseCollectedCount` _array_element)
      (`self.K2_DestroyActor`))))

(fn `UserConstructionScript`)